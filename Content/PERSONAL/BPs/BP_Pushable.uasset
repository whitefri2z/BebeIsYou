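; BP_Pushable is a pushable pawn that appears as an item type such as tree, rock or Bibi statue.
; The construction script picks the mesh from the item enum, or shows a cube with the type's name when IsText is set.
; Move rejects diagonal input and uses AI MoveTo to step by Movement from its location, mapping Y input to world X and X to world Y.
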(event `self.ReceiveBeginPlay`)

(event `Move`
  (params (X :type "Float (double-precision)") (Y :type "Float (double-precision)"))
  (bind _movement (`self.movement`))
  (bind (_returnvalue_x _returnvalue_y _returnvalue_z) (`KismetMathLibrary.BreakVector` (`SceneComponent.K2_GetComponentLocation` (`self.Scene`))))
  (if (not (and (!= X 0.0) (!= Y 0.0)))
    (`|AIMoveTo` self (`KismetMathLibrary.MakeVector` (+ _returnvalue_x (* Y _movement)) (+ _returnvalue_y (* X _movement)) _returnvalue_z) null
      (:`OnSuccess`
        (`KismetSystemLibrary.PrintString` "Hello")))))

(fn `UserConstructionScript`
  (locals (`Text:None` :type Text))
  (bind _istext (`self.IsText`))
  (`StaticMeshComponent.SetStaticMesh` (`self.StaticMesh`) (select `bool` _istext :`false` (select `/Game/PERSONAL/Enums/Enum_StaticMeshesType` (`self.Enum_ItemType`) :`NewEnumerator0` "/Game/StarterContent/Shapes/Shape_Cube.Shape_Cube" :`NewEnumerator2` "/Game/StarterContent/Props/SM_Rock.SM_Rock" :`NewEnumerator3` "/Game/StarterContent/Props/SM_Statue.SM_Statue" :!type "StaticMesh Object Reference") :`true` "/Game/StarterContent/Shapes/Shape_Cube.Shape_Cube"))
  (if _istext
    (`TextRenderComponent.K2_SetText` (`self.TextRender`) (select `/Game/PERSONAL/Enums/Enum_StaticMeshesType` (`self.Enum_ItemType`) :`NewEnumerator0` "Why you \nseeing this?" :`NewEnumerator1` "TREE" :`NewEnumerator2` "ROCK" :`NewEnumerator3` "BIBI" :!type "Text"))
    (else
      (`TextRenderComponent.K2_SetText` (`self.TextRender`) (`local.Text:None`)))))